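; A door Blueprint that swings open while enough mass rests on a linked pressure plate and closes when it does not.
; Each overlap change on the plate sums the mesh masses of overlapping actors, printing the total, and compares it to a threshold.
; A state flag fires start and stop events only on transitions.
; These play or reverse a timeline that yaws the door from its initial rotation and triggers a lock sound.
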(event Custom|OnTriggerStart
  ;[1 1 1] Open the door on Trigger Start
  (CallFunction|OpentheDoor))

(event Custom|OnTriggerStop
  ;[1 1 1] Close th door on trigger Stop
  (CallFunction|ClosetheDoor))

(event OnActorBeginOverlap(PressurePlate)
  (params (OverlappedActor :type Actor%20Object%20Reference) (OtherActor :type Actor%20Object%20Reference))
  ;[1 1 1] Call events on overlap change, when actor stop or start overlapping the trigger
  (CallFunction|OnOverlapChange))

(event OnActorEndOverlap(PressurePlate)
  (params (OverlappedActor :type Actor%20Object%20Reference) (OtherActor :type Actor%20Object%20Reference))
  ;[1 1 1] Call events on overlap change, when actor stop or start overlapping the trigger
  (CallFunction|OnOverlapChange))

(event Custom|OnOverlapChange
  ;[1 1 1] On Overlap Change, test if trigger change, then call events on trigger start, on trigger stop
  (bind _istriggered (PressurePlate|IsTriggered))
  (if _istriggered
    (if (not (Variables|Default|GetIsTriggerd))
      (Variables|Default|SetIsTriggerd true)
      (CallFunction|OnTriggerStart))
    (elif (Variables|Default|GetIsTriggerd)
      (Variables|Default|SetIsTriggerd false)
      (CallFunction|OnTriggerStop))))

(event Custom|OpenTheDoor
  ;[1 1 1] Control the aperture of the door, play a sound when the door is closed
  (bind _door_aperture_in_degree (Timeline|Timeline_0 Play)
    (:Update
      (Transformation|SetWorldRotation (Variables|Debug|GetStaticMeshComponent) (Math|Rotator|CombineRotators (Variables|Default|GetInitialDoorRotation) (Math|Rotator|MakeRotator 0.0 0.0 _door_aperture_in_degree)) false false))
    (:PlayLockSound
      (Audio|PlaySoundatLocation "/Game/door-lock.door-lock" (Transformation|GetWorldLocation (Variables|Debug|GetStaticMeshComponent)) "0, 0, 0" 1.0 1.0 0.0 0 0 0))))

(event Custom|CloseTheDoor
  ;[1 1 1] Control the aperture of the door, play a sound when the door is closed
  (bind _door_aperture_in_degree (Timeline|Timeline_0 Reverse)
    (:Update
      (Transformation|SetWorldRotation (Variables|Debug|GetStaticMeshComponent) (Math|Rotator|CombineRotators (Variables|Default|GetInitialDoorRotation) (Math|Rotator|MakeRotator 0.0 0.0 _door_aperture_in_degree)) false false))
    (:PlayLockSound
      (Audio|PlaySoundatLocation "/Game/door-lock.door-lock" (Transformation|GetWorldLocation (Variables|Debug|GetStaticMeshComponent)) "0, 0, 0" 1.0 1.0 0.0 0 0 0))))

(event EventBeginPlay
  ;[1 1 1] Save initial world location of the door in variable "Initial Door Location"
  (Variables|Default|SetInitialDoorRotation (Transformation|GetWorldRotation (Variables|Debug|GetStaticMeshComponent))))

(fn ConstructionScript)

(fn IsTriggered
  (bind _totalmass (PressurePlate|GetOverlapMass (Variables|OpeningSystem|GetPressurePlate)))
  (return (> _totalmass (Variables|OpeningSystem|GetTotalMassInkgToTrigger))))

(fn GetOverlapMass
  (params (Actor :type Actor%20Object%20Reference))
  ;[1 1 1] Return the total mass of all the objects that are overlapping an actor
  (LocalVariables|SetTmpTotalMass 0.0)
  (for _array_element (Collision|GetOverlappingActors Actor 0 :!class /Script/Engine.Actor)
    (for _array_element_2 (Actor|GetComponentsByClass _array_element "/Script/Engine.MeshComponent")
      (LocalVariables|SetTmpTotalMass (+ (LocalVariables|GetTmpTotalMass) (Physics|GetMass _array_element_2)))))
  (Development|PrintString (Utilities|String|ToString(Float) (LocalVariables|GetTmpTotalMass)))
  (return (LocalVariables|GetTmpTotalMass)))